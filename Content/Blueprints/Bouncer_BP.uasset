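; Bouncer Blueprint that launches the player character high into the air when triggered within its box area.
; Box overlap toggles a CanLaunch flag and sets CanInteract on the ThirdPersonCharacter.
; The LaunchPlayer event, when allowed, launches player pawn zero upward at a multiple of its jump Z velocity, overriding current vertical speed.
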(event `self.Box Area.OnComponentBeginOverlap`
  (params (OverlappedComponent :type "PrimitiveComponent Object Reference") (OtherActor :type "Actor Object Reference") (OtherComp :type "PrimitiveComponent Object Reference") (OtherBodyIndex :type Integer) (bFromSweep :type Boolean) (SweepResult :type "HitResult Structure (by ref)"))
  (bind _asthird_person_character (cast `/Game/ThirdPersonBP/Blueprints/ThirdPersonCharacter` OtherActor))
  (set `/Game/ThirdPersonBP/Blueprints/ThirdPersonCharacter.CanInteract` true _asthird_person_character)
  (set `self.CanLaunch` true))

(event `self.Box Area.OnComponentEndOverlap`
  (params (OverlappedComponent :type "PrimitiveComponent Object Reference") (OtherActor :type "Actor Object Reference") (OtherComp :type "PrimitiveComponent Object Reference") (OtherBodyIndex :type Integer))
  (bind _asthird_person_character (cast `/Game/ThirdPersonBP/Blueprints/ThirdPersonCharacter` OtherActor))
  (set `/Game/ThirdPersonBP/Blueprints/ThirdPersonCharacter.CanInteract` false _asthird_person_character)
  (set `self.CanLaunch` false))

(event `Launch Player`
  (if (`self.CanLaunch`)
    (bind _asthird_person_character (cast `/Game/ThirdPersonBP/Blueprints/ThirdPersonCharacter` (`GameplayStatics.GetPlayerPawn` 0)))
    (`Character.LaunchCharacter` _asthird_person_character (`KismetMathLibrary.MakeVector` 0.0 0.0 (* (`CharacterMovementComponent.JumpZVelocity` (`Character.CharacterMovement` _asthird_person_character)) 3.0)) false true)))

(fn `UserConstructionScript`)